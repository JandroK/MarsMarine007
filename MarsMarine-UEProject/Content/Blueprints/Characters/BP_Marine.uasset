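; Player marine character for what appears to be a top-down shooter, handling movement, aiming, rifle fire, health and HUD.
; Each tick it aims by gamepad stick, cursor hit or mouse-delta virtual joystick, switched by key presses or middle mouse.
; Firing loops a timer-driven line trace from the muzzle, leveled at weapon height for mouse aim.
; Damage flashes blood on screen; death disables input, then shows the lose screen and saves via BP_GameMode.
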(event EventBeginPlay
  ;[0.3369 1 0.4858 0.255] Create HUD
  (bind _returnvalue (SaveGame|LoadGamefromSlot "killcount"))
  (bind _assg_game_data (Utilities|Casting|CastToSG_GameData _returnvalue))
  (bind _returnvalue_2 (UserInterface|CreateWidget "/Game/UI/W_PlayerHUD.W_PlayerHUD_C" 0 self (Variables|/Game/Blueprints/SG_GameData.SG_GameData_C|GetKill%20Record _assg_game_data)))
  (UserInterface|Viewport|AddtoViewport _returnvalue_2 0)
  (bind _returnvalue_3 (UserInterface|CreateWidget "/Game/UI/W_BloodEffect.W_BloodEffect_C"))
  (Variables|Default|SetHUD%20Blood _returnvalue_3)
  (UserInterface|Viewport|AddtoViewport _returnvalue_3 0))

(event EventTick
  (params (DeltaSeconds :type Float%20%28single-precision%29))
  ;[0.2687 0.998 1 0.317] Update Aim Direction
  (if (Health|IsAlive)
    (CallFunction|UpdateAim)))

(event Game|Damage|EventAnyDamage
  (params (Damage :type Float%20%28single-precision%29) (DamageType :type Damage%20Type%20Object%20Reference) (InstigatedBy :type Controller%20Object%20Reference) (DamageCauser :type Actor%20Object%20Reference))
  ;[1 0 0.001906 0.417] Apply Damage - Dead Condition
  (bind _health (Health|DecreaseHealth Damage))
  (if (== _health 0.0)
    (Variables|Stats|SetDying true)
    (Input|DisableInput (Game|GetPlayerController 0))
    (Weapon|StopFiring)
    (Utilities|FlowControl|Delay 1.2)
    (CallFunction|ToLoseScene)))

(event Input|ActionEvents|InputActionFireWeapon
  (params (Key :type Key%20Structure :default "None"))
  ;[1 0.1758 0 0.292] Shoot
  (:Pressed
    (Weapon|StartFiring))
  (:Released
    (Weapon|StopFiring)))

(event Input|AxisEvents|InputAxisMoveForward/Backward
  (params (AxisValue :type Float%20%28single-precision%29))
  ;[1 1 1 0.229] Player Movement
  (Pawn|Input|AddMovementInput "1.000000, 0, 0" AxisValue false))

(event Input|AxisEvents|InputAxisMoveRight/Left
  (params (AxisValue :type Float%20%28single-precision%29))
  ;[1 1 1 0.229] Player Movement
  (Pawn|Input|AddMovementInput "0,1.000000, 0" AxisValue false))

(event Input|KeyboardEvents|R
  (params (Key :type Key%20Structure :default "None"))
  ;[0.1205 0.697 1 0.421] Restart Record - Debug
  (:Pressed
    (bind _asbp_game_mode (Utilities|Casting|CastToBP_GameMode (Game|GetGameMode)))
    (Default|RestartRecord _asbp_game_mode)))

(event Input|KeyboardEvents|Escape
  (params (Key :type Key%20Structure :default "None"))
  ;[1 1 1] Quit Game
  (:Pressed
    (Game|QuitGame (Game|GetPlayerController 0) "Quit" false)))

(event Input|KeyboardEvents|AnyKey
  (params (Key :type Key%20Structure :default "None"))
  ;[1 0.5868 0.1546 0.354] Input Controller
  (:Pressed
    (if (Class|KismetInputLibrary|KeyIsGamepadKey Key)
      (Variables|Default|SetInput%20Control "NewEnumerator0")
      (CallFunction|SetShowCursor false)
      (elif (Utilities|Enum|Equal(Enum) (Variables|Default|GetInput%20Control) "NewEnumerator0")
        (Variables|Default|SetInput%20Control "NewEnumerator1")
        (CallFunction|SetShowCursor true)))))

(event Input|MouseEvents|MiddleMouseButton
  (params (Key :type Key%20Structure :default "None"))
  ;[1 0.5868 0.1546 0.354] Input Controller
  (:Pressed
    (if (Utilities|Enum|Equal(Enum) (Variables|Default|GetInput%20Control) "NewEnumerator1")
      (Variables|Default|SetInput%20Control "NewEnumerator2")
      (CallFunction|SetShowCursor false)
      (else
        (Variables|Default|SetInput%20Control "NewEnumerator1")
        (CallFunction|SetShowCursor true)))))

(fn ConstructionScript)

(fn UpdateAim
  (switch Utilities|FlowControl|Switch|SwitchonEnum_InputControlers (Variables|Default|GetInput%20Control)
    (:NewEnumerator0
      (if (AimGamepad|IsOutOfDeadZoneGamePad)
        (AimGamepad|AimPlayer(GamePad))))
    (:NewEnumerator1
      (AimMouse|AimPlayer(Mouse)))
    (:NewEnumerator2
      (if (AimJoystick|IsOutOfDeadZoneJoystick)
        (AimJoystick|AimPlayer(Joystick))))))

(fn AimPlayer(Joystick)
  (bind _returnvalue (Game|GetPlayerController 0))
  (Pawn|SetControlRotation _returnvalue (Math|Interpolation|RInterpTo (Pawn|GetControlRotation _returnvalue :!class /Script/Engine.Controller) (AimJoystick|GetJoystickDirection) (Utilities|Time|GetWorldDeltaSeconds) (Variables|Default|GetAngular%20Speed%20%28Degrees%29))))

(fn AimPlayer(GamePad)
  (bind _returnvalue (Game|GetPlayerController 0))
  (Pawn|SetControlRotation _returnvalue (Math|Interpolation|RInterpTo (Pawn|GetControlRotation _returnvalue :!class /Script/Engine.Controller) (AimGamepad|GetGamepadDirection) (Utilities|Time|GetWorldDeltaSeconds) (Variables|Default|GetAngular%20Speed%20%28Degrees%29))))

(fn GetJoystickDirection
  (bind _returnvalue (AimJoystick|MouseVelocity))
  (return (Math|Rotator|MakeRotator 0.0 0.0 (Class|KismetMathLibrary|DegAtan2 (.x _returnvalue) (.y _returnvalue)))))

(fn IsOutOfDeadZoneJoystick
  (return (> (Math|Vector2D|Vector2DLength (AimJoystick|MouseVelocity)) (LocalVariables|GetRadius%20DeadZone))))

(fn GetGamepadDirection
  (return (Math|Rotator|MakeRotator 0.0 0.0 (Class|KismetMathLibrary|DegAtan2 (Input|AxisValues|GetThumbstickAimingRight/Left) (Input|AxisValues|GetThumbstickAimingUp/Down)))))

(fn IsOutOfDeadZoneGamePad
  (return (> (Math|Vector2D|Vector2DLength (Math|Vector2D|MakeVector2D (Input|AxisValues|GetThumbstickAimingRight/Left) (Input|AxisValues|GetThumbstickAimingUp/Down))) (LocalVariables|GetRadius%20DeadZone))))

(fn MouseVelocity
  (bind _returnvalue (Utilities|Time|GetWorldDeltaSeconds))
  (bind _returnvalue_2 (Game|GetPlayerController 0))
  (bind (_deltax _deltay) (Class|PlayerController|GetInputMouseDelta _returnvalue_2))
  (return (/ (Math|Vector2D|MakeVector2D _deltax _deltay) (Math|Vector2D|MakeVector2D _returnvalue _returnvalue))))

(fn AimPlayer(Mouse)
  (bind _returnvalue (Transformation|GetActorLocation))
  (bind _location (AimMouse|GetMouseLocation))
  (Pawn|SetControlRotation (Game|GetPlayerController 0) (Math|Rotator|FindLookatRotation (Math|Vector|MakeVector (.x _returnvalue) (.y _returnvalue) (.z _returnvalue)) (Math|Vector|MakeVector (.x _location) (.y _location) (.z _returnvalue)))))

(fn GetMouseLocation
  (return (.impactpoint (.HitResult (Game|Player|GetHitResultUnderCursorbyChannel (Game|GetPlayerController 0) "TraceTypeQuery1" false)))))

(fn SetShowCursor
  (params (bool :type Boolean))
  (bind _returnvalue (Game|GetPlayerController 0))
  (if (!= bool (Variables|/Script/Engine.PlayerController|GetbShowMouseCursor _returnvalue))
    (Variables|/Script/Engine.PlayerController|SetbShowMouseCursor _returnvalue bool)))

(fn StartFiring
  (Components|Activation|SetActive (Variables|Default|GetP_AssaultRifle_MF) true false)
  (bind _returnvalue (Audio|SpawnSound2D "/Game/Sounds/Weapon_AssaultRifle/Stereo/RifleShoot_Cue.RifleShoot_Cue" 1.0 1.0 0.0 0))
  (Variables|Default|SetSoundShoot _returnvalue)
  (Weapon|WeaponTrace)
  (Utilities|Time|SetTimerbyFunctionName 0 "Weapon Trace" (Variables|Stats|GetShot%20Rate) true))

(fn StopFiring
  (bind _soundshoot (Variables|Default|GetSoundShoot))
  (Components|Activation|SetActive (Variables|Default|GetP_AssaultRifle_MF) false false)
  (Utilities|IsValid _soundshoot
    (:Is%20Valid
      (Audio|Components|Audio|Stop _soundshoot))
    (:Is%20Not%20Valid
      _))
  (Utilities|Time|ClearTimerbyFunctionName 0 "Weapon Trace")
  (if (Health|IsAlive)
    (Audio|SpawnSound2D "/Game/Sounds/Weapon_AssaultRifle/Stereo/RifleShootEnd_Cue.RifleShootEnd_Cue" 1.0 1.0 0.0 0)))

(fn IsAlive
  (return (not (Variables|Stats|GetDying))))

(fn DecreaseHealth
  (params (Damage%20Amount :type Float%20%28double-precision%29))
  (bind _output_get (Variables|Stats|SetHealth (Math|Float|Clamp(Float) (- (Variables|Stats|GetHealth) Damage%20Amount) 0.0 1e+02)))
  (CallFunction|SpwanHUDBlood)
  (return _output_get))

(fn WeaponTrace
  (bind _outhit (Collision|LineTraceByChannel (Weapon|StartWeaponTrace) (Weapon|EndWeaponTrace) "TraceTypeQuery1" false 0 "ForDuration" true "(R=1.000000,G=0.000000,B=0.000000,A=1.000000)" "(R=0.000000,G=1.000000,B=0.000000,A=1.000000)" 2.0))
  (if (.bBlockingHit (Collision|BreakHitResult _outhit))
    (Weapon|SpawnImpactHit (.Location (Collision|BreakHitResult _outhit)))
    (Game|Damage|ApplyDamage (.HitActor (Collision|BreakHitResult _outhit)) (Variables|Stats|GetDamage%20per%20hit) 0 0)))

(fn StartWeaponTrace
  (return (Transformation|GetSocketLocation (Variables|Default|GetWeapon) "MuzzleFlashSocket")))

(fn EndWeaponTrace
  (bind _returnvalue (AimGamepad|GetThumbstickEndTrace))
  (return (Utilities|Select :Index (Variables|Default|GetInput%20Control) :NewEnumerator0 _returnvalue :NewEnumerator1 (AimMouse|GetMouseEndTrace) :NewEnumerator2 _returnvalue)))

(fn SpawnImpactHit
  (params (Location :type Vector))
  (Effects|SpawnEmitteratLocation "/Game/Effects/Weapons/Impacts/P_AssaultRifle_IH.P_AssaultRifle_IH" Location))

(fn IsHealthFull
  (return (== (Variables|Stats|GetHealth) 1e+02)))

(fn RecoverHealth
  (params (Health%20to%20Add :type Float%20%28double-precision%29))
  (Variables|Stats|SetHealth (Math|Float|Clamp(Float) (+ Health%20to%20Add (Variables|Stats|GetHealth)) 0.0 1e+02)))

(fn ToLoseScene
  (bind _returnvalue (UserInterface|CreateWidget "/Game/UI/W_PlayerLose.W_PlayerLose_C" 0 self))
  (UserInterface|Viewport|AddtoViewport _returnvalue 0)
  (Class|UserWidget|PlayAnimationForward _returnvalue (Variables|/Game/UI/W_PlayerLose.W_PlayerLose_C|GetFadeIn _returnvalue) 1.0 false)
  (bind _asbp_game_mode (Utilities|Casting|CastToBP_GameMode (Game|GetGameMode)))
  (Default|SaveGame _asbp_game_mode)
  (Default|ChangeAudiotoLose _asbp_game_mode))

(fn GetKillRecord
  (bind _asbp_game_mode (Utilities|Casting|CastToBP_GameMode (Game|GetGameMode)))
  (return (Variables|/Game/Blueprints/BP_GameMode.BP_GameMode_C|GetKill%20Record _asbp_game_mode)))

(fn GetHeighWeapon
  (return (.z (Weapon|StartWeaponTrace))))

(fn GetMouseEndTrace
  (bind _location (AimMouse|GetMouseLocation))
  (bind _returnvalue (Weapon|StartWeaponTrace))
  (return (+ (* (Math|Vector|Normalize (- (Math|Vector|MakeVector (.x _location) (.y _location) (Weapon|GetHeighWeapon)) _returnvalue)) 5000) _returnvalue)))

(fn GetThumbstickEndTrace
  (return (+ (Weapon|StartWeaponTrace) (* (Math|Vector|GetForwardVector (Pawn|GetControlRotation :!class /Script/Engine.Pawn)) 5000))))

(fn SpwanHUDBlood
  (bind _hud_blood (Variables|Default|GetHUD%20Blood))
  (bind _hud_blood_2 (Variables|Default|GetHUD%20Blood))
  (bind _opacitydown (Variables|/Game/UI/W_BloodEffect.W_BloodEffect_C|GetOpacityDown _hud_blood))
  (if (Class|UserWidget|IsAnimationPlaying _hud_blood_2 (Variables|/Game/UI/W_BloodEffect.W_BloodEffect_C|GetOpacityDown _hud_blood_2))
    (Class|UserWidget|SetAnimationCurrentTime _hud_blood _opacitydown 0.0))
  (Class|UserWidget|PlayAnimationForward _hud_blood _opacitydown 1.0 false))