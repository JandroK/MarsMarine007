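; BP_Alien is a spider enemy character that chases the player marine and attacks in melee.
; An AI MoveTo loop plays a random attack montage on arrival, with its "Attack" notify applying damage if the player is still in range.
; Lethal damage disables movement and collision and credits the marine's kill count.
; After a delay, Tick shrinks the mesh, removes the alien from the GameMode list and destroys it.
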(event EventBeginPlay
  ;[1 0.6039 0.03756 0.35] AI Movement
  (CallFunction|InitPlayer)
  (AI|AIMoveTo self "0, 0, 0" (Game|GetPlayerCharacter 0) (Variables|Default|GetAttack%20Range) false :!label _label
    (:OnSuccess
      (if (CallFunction|CanAttack)
        (bind _notifyname (Animation|Montage|PlayMontage (Variables|Character|GetMesh) (CallFunction|PlayRandomAttackAnim))
          (:OnCompleted
            (goto _label))
          (:OnNotifyBegin
            (CallFunction|AttackCharacter _notifyname)))))
    (:OnFail
      (goto _label))))

(event EventTick
  (params (DeltaSeconds :type Float%20%28single-precision%29))
  ;[1 0.1939 0.9918 0.283] Post-Dead
  (if (Utilities|Enum|Equal(Enum) (Variables|Default|GetState) "NewEnumerator2")
    (DeadState|ToDisappear)
    (Utilities|FlowControl|Delay 1.0)
    (CallFunction|RemoveAlienfromList)
    (Actor|DestroyActor)))

(event Game|Damage|EventAnyDamage
  (params (Damage :type Float%20%28single-precision%29) (DamageType :type Damage%20Type%20Object%20Reference) (InstigatedBy :type Controller%20Object%20Reference) (DamageCauser :type Actor%20Object%20Reference))
  ;[1 0 0.02458 0.321] Apply Damage - Dead Condition
  (CallFunction|ReceiveDamage Damage)
  (if (CallFunction|IsDead)
    (Utilities|FlowControl|DoOnce false
      (:Completed
        (DeadState|KillAI)
        (Utilities|FlowControl|Delay 1.8)
        (Variables|Default|SetState "NewEnumerator2")))))

(fn ConstructionScript)

(fn AttackCharacter
  (params (Event%20Name :type Name))
  (if (and (== Event%20Name "Attack") (CallFunction|IsPlayeronRange))
    (Game|Damage|ApplyDamage (Game|GetPlayerCharacter 0) 1e+01 0 0)))

(fn PlayRandomAttackAnim
  (return (Utilities|Select :Index (Math|Random|RandomIntegerinRange 0 2) :Option%200 "/Game/Characters/Enemy_Great_Spider/Animations/ExoGame_Greater_Spider_Attack_Melee_A_Montage.ExoGame_Greater_Spider_Attack_Melee_A_Montage" :Option%201 "/Game/Characters/Enemy_Great_Spider/Animations/ExoGame_Greater_Spider_Attack_Melee_B_Montage.ExoGame_Greater_Spider_Attack_Melee_B_Montage" :Option%202 "/Game/Characters/Enemy_Great_Spider/Animations/ExoGame_Greater_Spider_Attack_Melee_C_Montage.ExoGame_Greater_Spider_Attack_Melee_C_Montage")))

(fn IsPlayeronRange
  (return (<= (Transformation|GetDistanceTo (Game|GetPlayerCharacter 0)) (+ (Variables|Default|GetAttack%20Range) (LocalVariables|GetOffset)))))

(fn ReceiveDamage
  (params (Damage :type Float%20%28double-precision%29))
  (Variables|Default|SetHealth (- (Variables|Default|GetHealth) Damage)))

(fn IsDead
  (return (<= (Variables|Default|GetHealth) 0.0)))

(fn IsAlive
  (return (Utilities|Enum|Equal(Enum) (Variables|Default|GetState) "NewEnumerator0")))

(fn IfPlayingAnyMountageStopIt
  (if (Class|AnimInstance|IsAnyMontagePlaying (Components|SkeletalMesh|GetAnimInstance (Variables|Character|GetMesh)))
    (Animation|StopAnimMontage (Animation|GetCurrentMontage :!class /Script/Engine.Character)))
  (return))

(fn ToDisappear
  (Transformation|SetWorldScale3D (Variables|Character|GetMesh) (Math|Vector|Lerp(Vector) (Transformation|GetWorldScale (Variables|Character|GetMesh)) "0, 0, 0" 0.1)))

(fn IsDisappearComplete
  (return (<= (Math|Vector|VectorLength (Transformation|GetWorldScale (Variables|Character|GetMesh))) 0.0)))

(fn AddKill
  (bind _asbp_marine (Utilities|Casting|CastToBP_Marine (Game|GetPlayerCharacter 0)))
  (bind _result (Math|Integer|IncrementInt (Variables|/Game/Blueprints/Characters/BP_Marine.BP_Marine_C|GetKills _asbp_marine))
    (:%20%20
      (Variables|/Game/Blueprints/Characters/BP_Marine.BP_Marine_C|SetKills _asbp_marine _result))))

(fn KillAI
  (Variables|Default|SetState "NewEnumerator1")
  (Components|Activation|Deactivate (Variables|Character|GetCharacterMovement))
  (Collision|SetActorEnableCollision false)
  (DeadState|AddKill))

(fn RemoveAlienfromList
  (bind _asbp_game_mode (Utilities|Casting|CastToBP_GameMode (Game|GetGameMode)))
  (Utilities|Array|RemoveItem (Variables|/Game/Blueprints/BP_GameMode.BP_GameMode_C|GetAlien _asbp_game_mode) self))

(fn InitPlayer
  (bind _asbp_marine (Utilities|Casting|CastToBP_Marine (Game|GetPlayerCharacter 0)))
  (Variables|Default|SetMarine _asbp_marine))

(fn CanAttack
  (return (and (CallFunction|IsAlive) (Default|IsAlive (Variables|Default|GetMarine)))))