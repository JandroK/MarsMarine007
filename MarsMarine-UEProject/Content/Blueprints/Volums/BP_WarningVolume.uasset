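; BP_WarningVolume is a mission-area boundary that warns and punishes the player for leaving it.
; When a BP_Marine exits, it sets OutsideMissionArea and starts a five-second timer that damages player character 0; re-entering clears both.
; While outside, Tick replays a ping-pong red fade on the W_PlayerHUD widget, found shortly after BeginPlay, whenever that animation is not already playing.
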(event Collision|EventActorBeginOverlap
  (params (OtherActor :type Actor%20Object%20Reference))
  (bind _asbp_marine (Utilities|Casting|CastToBP_Marine OtherActor))
  (bind _output_get (Variables|/Game/Blueprints/Characters/BP_Marine.BP_Marine_C|SetOutside%20Mission%20Area _asbp_marine false))
  (Variables|Default|SetPlayer%20is%20outside _output_get)
  (Utilities|Time|ClearTimerbyFunctionName 0 "Kill Player"))

(event Collision|EventActorEndOverlap
  (params (OtherActor :type Actor%20Object%20Reference))
  (bind _asbp_marine (Utilities|Casting|CastToBP_Marine OtherActor))
  (bind _output_get (Variables|/Game/Blueprints/Characters/BP_Marine.BP_Marine_C|SetOutside%20Mission%20Area _asbp_marine true))
  (Variables|Default|SetPlayer%20is%20outside _output_get)
  (Utilities|Time|SetTimerbyFunctionName 0 "Kill Player" 5.0))

(event EventTick
  (params (DeltaSeconds :type Float%20%28single-precision%29))
  (if (Variables|Default|GetPlayer%20is%20outside)
    (CallFunction|StartWarningMessageAnimation)))

(event EventBeginPlay
  (Utilities|FlowControl|Delay 0.1)
  (bind _foundwidgets (Widget|GetAllWidgetsOfClass "/Game/UI/W_PlayerHUD.W_PlayerHUD_C" true))
  (Variables|Default|SetWidgetHUD (Utilities|Array|Get(acopy) _foundwidgets)))

(fn ConstructionScript)

(fn KillPlayer
  (Game|Damage|ApplyDamage (Game|GetPlayerCharacter 0) 1e+02 0 0))

(fn StartWarningMessageAnimation
  (bind _widgethud (Variables|Default|GetWidgetHUD))
  (bind _fadeinredalpha (Variables|/Game/UI/W_PlayerHUD.W_PlayerHUD_C|GetFadeInRedAlpha _widgethud))
  (if (not (Class|UserWidget|IsAnimationPlaying _widgethud _fadeinredalpha))
    (UserInterface|Animation|PlayAnimation (Variables|Default|GetWidgetHUD) _fadeinredalpha 0.0 1 "PingPong" 1.0 false)))