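; Game mode for a wave-based alien shooter that runs the waves, the kill record and the switch to lose music.
; A looping countdown starts each wave, spawning a health pickup and timed BP_Alien spawns at random TargetPoints until a wave-scaled total is reached.
; Tick restarts the countdown once the alien array empties.
; The best BP_Marine kill count persists through SG_GameData, with a reset that reloads the Mars level.
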(event EventBeginPlay
  (SaveLoad|LoadGame)
  (Utilities|Time|SetTimerbyFunctionName 0 "Decrease Countdown" 1.0 true)
  (CameraFades|StartCameraFade :self (Game|GetPlayerCameraManager 0) :FromAlpha 1.0 :Duration (Math|Float|MakeLiteralFloat 1.0) :bShouldFadeAudio true :bHoldWhenFinished true))

(event EventTick
  (params (DeltaSeconds :type Float%20%28single-precision%29))
  (if (Waves|NextWaveCondition)
    (Countdown|RestartCoundown)
    (Utilities|Time|SetTimerbyFunctionName 0 "Decrease Countdown" 1.0 true)))

(fn ConstructionScript)

(fn IncreaseWave
  (bind _result (Math|Integer|IncrementInt (Variables|Default|GetWave))
    (:%20%20
      (Variables|Default|SetWave _result))))

(fn DecreaseCountdown
  (bind _result (Math|Integer|DecrementInt (Variables|Default|GetCountdown))
    (:%20%20
      (bind _output_get (Variables|Default|SetCountdown _result))
      (if (== _output_get 0)
        (Waves|StartNextWave)))))

(fn StartNextWave
  (Utilities|Time|ClearTimerbyFunctionName 0 "Decrease Countdown")
  (Waves|IncreaseWave)
  (Spawn|SpawnHealthPickUp)
  (Spawn|SpawnAI)
  (Utilities|Time|SetTimerbyFunctionName 0 "Spawn AI" 0.6 true))

(fn SpawnAI
  (bind (_actor _location) (CallFunction|GetRandomTargetPosition))
  (Utilities|IsValid _actor
    (:Is%20Valid
      (bind _returnvalue (Game|SpawnActorfromClass "/Game/Blueprints/Characters/BP_Alien.BP_Alien_C" (Math|Transform|MakeTransform _location "0, 0, 0" "1.000000,1.000000,1.000000") "AlwaysSpawn" 0 0))
      (Utilities|Array|Add (Variables|Default|GetAlien) _returnvalue)
      (Spawn|EndSpawnAI))))

(fn EndSpawnAI
  (bind _result (Math|Integer|IncrementInt (Variables|Default|GetAlien%20Remaining))
    (:%20%20
      (if (== _result (Spawn|GetTotalAlienSpawn))
        (Utilities|Time|ClearTimerbyFunctionName 0 "Spawn AI")))))

(fn RestartCoundown
  (Variables|Default|SetCountdown 3)
  (Variables|Default|SetAlien%20Remaining 0))

(fn NextWaveCondition
  (return (and (Utilities|Array|IsEmpty (Variables|Default|GetAlien)) (== (Variables|Default|GetCountdown) 0))))

(fn GetRandomTargetPosition
  (bind _outactors (Actor|GetAllActorsOfClass "/Script/Engine.TargetPoint"))
  (return (Utilities|Array|Get(acopy) _outactors (Math|Random|RandomIntegerinRange 0 (Utilities|Array|LastIndex _outactors))) (Transformation|GetActorLocation (Utilities|Array|Get(acopy) _outactors (Math|Random|RandomIntegerinRange 0 (Utilities|Array|LastIndex _outactors))))))

(fn GetTotalAlienSpawn
  (return (Math|Float|Truncate (* (Variables|Default|GetWave) (Variables|Default|GetWave%20difficult) (LocalVariables|GetAlien%20in%20First%20Wave)))))

(fn SpawnHealthPickUp
  (bind (_actor _location) (CallFunction|GetRandomTargetPosition))
  (Utilities|IsValid _actor
    (:Is%20Valid
      (Game|SpawnActorfromClass "/Game/Blueprints/PickUps/BP_HealthPickUp.BP_HealthPickUp_C" (Math|Transform|MakeTransform _location "0, 0, 0" "1.000000,1.000000,1.000000") "Undefined" 0 0))))

(fn SaveGame
  (bind _returnvalue (SaveGame|CreateSaveGameObject "/Game/Blueprints/SG_GameData.SG_GameData_C"))
  (Variables|/Game/Blueprints/SG_GameData.SG_GameData_C|SetKill%20Record _returnvalue (CallFunction|GetMaxKillCount))
  (SaveGame|SaveGametoSlot _returnvalue "killcount"))

(fn LoadGame
  (bind _returnvalue (SaveGame|LoadGamefromSlot "killcount"))
  (bind _assg_game_data (Utilities|Casting|CastToSG_GameData _returnvalue))
  (Variables|Default|SetKill%20Record (Variables|/Game/Blueprints/SG_GameData.SG_GameData_C|GetKill%20Record _assg_game_data)))

(fn GetCurrentKills
  (bind _asbp_marine (Utilities|Casting|CastToBP_Marine (Game|GetPlayerCharacter 0)))
  (return (Variables|/Game/Blueprints/Characters/BP_Marine.BP_Marine_C|GetKills _asbp_marine)))

(fn IsRecordBroken
  (return (> (CallFunction|GetCurrentKills) (Variables|Default|GetKill%20Record))))

(fn RestartRecord
  (bind _returnvalue (SaveGame|CreateSaveGameObject "/Game/Blueprints/SG_GameData.SG_GameData_C"))
  (Variables|/Game/Blueprints/SG_GameData.SG_GameData_C|SetKill%20Record _returnvalue 0)
  (SaveGame|SaveGametoSlot _returnvalue "killcount")
  (Game|OpenLevel(byName) "Mars"))

(fn GetMaxKillCount
  (if (CallFunction|IsRecordBroken)
    (return (CallFunction|GetCurrentKills))
    (else
      (return (Variables|Default|GetKill%20Record)))))

(fn ChangeAudiotoLose
  (bind _returnvalue (Math|Float|MakeLiteralFloat 1.0))
  (Audio|Components|Audio|FadeOut (Variables|Default|GetAudio) _returnvalue 0.0 "Linear" :!class /Script/Engine.AudioComponent)
  (Utilities|Time|SetTimerbyFunctionName 0 "Set Lose Sound" _returnvalue))

(fn SetLoseSound
  (bind _audio (Variables|Default|GetAudio))
  (Audio|Components|Audio|SetSound _audio "/Game/Sounds/Music/ShooterGame_Music_Intro_Cue.ShooterGame_Music_Intro_Cue")
  (Audio|Components|Audio|Play _audio 0.0))